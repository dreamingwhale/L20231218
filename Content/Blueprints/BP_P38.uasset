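; BP_P38 is a player-flown P-38 plane pawn that fires homing rockets.
; It moves forward every tick at a speed switched by boost and decelerate inputs, while Enhanced Input drives local pitch and roll.
; Propeller meshes register with a rotation component on BeginPlay.
; Firing spawns BP_Rocket at the Arrow, homes it on the second player's P-38 Box, and attaches a particle emitter.
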(event `self.ReceiveBeginPlay`
  ;[1 1 1] 컴포넌트 추가
  (`/Game/Blueprints/BP_PropellerRotation.AddRight` (`self.BP_PropellerRotation`) (`self.SM_P38_Propeller_Right`))
  (`/Game/Blueprints/BP_PropellerRotation.AddLeft` (`self.BP_PropellerRotation`) (`self.SM_P38_Propeller_Left`))
  (`KismetSystemLibrary.Delay` 3.0)
  (set `self.IsHomingProjectile` true))

(event `InputAction|Boost`
  (params (Key :type "Key Structure"))
  (:`Pressed`
    (set `self.Speed` 1.0))
  (:`Released`
    (set `self.Speed` 0.5)))

(event `self.ReceiveTick`
  (params (DeltaSeconds :type "Float (single-precision)"))
  (`self.AddMovementInput` (* (`self.GetActorForwardVector`) (`self.Speed`))))

(event `InputAction|DecreaseSpeed`
  (params (Key :type "Key Structure"))
  (:`Pressed`
    (set `self.Speed` 0.2))
  (:`Released`
    (set `self.Speed` 0.5)))

(event `EnhancedInput|/Game/Blueprints/Input/IA_PitchAndRoll`
  (params (ActionValue :type "Vector2D Structure") (ElapsedSeconds :type "Float (double-precision)") (TriggeredSeconds :type "Float (double-precision)") (InputAction :type "InputAction Object Reference" :default "/Game/Blueprints/Input/IA_PitchAndRoll.IA_PitchAndRoll"))
  (:`Triggered`
    (`self.K2_AddActorLocalRotation` (`KismetMathLibrary.MakeRotator` 0.0 (* ActionValue_Y (`self.RotateSpeed`) (`GameplayStatics.GetWorldDeltaSeconds`))))
    (`self.K2_AddActorLocalRotation` (`KismetMathLibrary.MakeRotator` (* ActionValue_X (`self.RotateSpeed`) (`GameplayStatics.GetWorldDeltaSeconds`))))))

(event `EnhancedInput|/Game/Blueprints/Input/IA_Fire`
  (params (ActionValue :type Boolean) (ElapsedSeconds :type "Float (double-precision)") (TriggeredSeconds :type "Float (double-precision)") (InputAction :type "InputAction Object Reference" :default "/Game/Blueprints/Input/IA_Fire.IA_Fire"))
  ;[1 1 1] 미사일 발사
  (:`Triggered`
    (bind _returnvalue (`|SpawnActorFromClass` "/Game/Blueprints/BP_Rocket.BP_Rocket_C" (`SceneComponent.K2_GetComponentToWorld` (`self.Arrow`)) "AlwaysSpawn" "MultiplyWithRoot" null null))
    (`|ExecutionSequence`
      (:`then_0`
        (bind _asbp_p38 (cast `/Game/Blueprints/BP_P38` (`GameplayStatics.GetPlayerPawn` 1)))
        (`/Game/Blueprints/BP_Rocket.Event_HomingMissile` _returnvalue (`/Game/Blueprints/BP_P38.Box` _asbp_p38)))
      (:`then_1`
        (bind _asbp_rocket (cast `/Game/Blueprints/BP_Rocket` _returnvalue))
        (`GameplayStatics.SpawnEmitterAttached` "/Engine/Tutorial/SubEditors/TutorialAssets/TutorialParticleSystem.TutorialParticleSystem" (`/Game/Blueprints/BP_Rocket.StaticMesh` _asbp_rocket) "None" (0.0 0.0 0.0) (struct) (0.2 0.2 0.2))))))

(fn `UserConstructionScript`)