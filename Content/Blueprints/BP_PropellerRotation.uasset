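; Propeller rotation Blueprint that spins registered scene components with a gradual spin-up.
; Each Tick compounds Speed by a delta-time-scaled fraction of itself, stopping short of exceeding MaxSpeed, so it needs a non-zero starting value to accelerate.
; AddLeft and AddRight fill two component arrays, which roll in opposite local directions at that shared, frame-time-scaled speed.
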(event `self.ReceiveTick`
  (params (DeltaSeconds :type "Float (single-precision)"))
  (bind _speed (`self.Speed`))
  (bind _returnvalue (+ _speed (* DeltaSeconds _speed)))
  (`|ExecutionSequence`
    (:`then_0`
      (if (<= _returnvalue (`self.MaxSpeed`))
        (set `self.Speed` _returnvalue)))
    (:`then_1`
      (for _array_element (`self.SceneComponentLeft`)
        (`SceneComponent.K2_AddLocalRotation` _array_element (`KismetMathLibrary.MakeRotator` (* (`self.Speed`) 1.0 (`GameplayStatics.GetWorldDeltaSeconds`))) false false)))
    (:`then_2`
      (for _array_element_2 (`self.SceneComponentRight`)
        (`SceneComponent.K2_AddLocalRotation` _array_element_2 (`KismetMathLibrary.MakeRotator` (* (`self.Speed`) -1.0 (`GameplayStatics.GetWorldDeltaSeconds`))) false false)))))

(fn `AddLeft`
  (params (SceneComponent :type "SceneComponent Object Reference"))
  (`KismetArrayLibrary.Array_Add` (`self.SceneComponentLeft`) SceneComponent))

(fn `AddRight`
  (params (SceneComponentRight :type "SceneComponent Object Reference"))
  (`KismetArrayLibrary.Array_Add` (`self.SceneComponentRight`) SceneComponentRight))